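; Example trigger actor that shows a widget on the game UI layer when a BP_Character enters its box.
; Begin overlap finds the player controller through PlayerState, pushes W_Example onto its activatable stack layer and fills it with a configurable count of W_Dummy widgets.
; Each dummy's ViewModel, using the "Create Instance" creation type, receives its index as DummyNum.
; An end-overlap handler, noted as example only, clears and removes the widget.
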(event OnComponentBeginOverlap(Box)
  (params (OverlappedComponent :type Primitive%20Component%20Object%20Reference) (OtherActor :type Actor%20Object%20Reference) (OtherComp :type Primitive%20Component%20Object%20Reference) (OtherBodyIndex :type Integer) (bFromSweep :type Boolean) (SweepResult :type Hit%20Result%20Structure%20%28by%20ref%29))
  (bind _asbp_character (Utilities|Casting|CastToBP_Character OtherActor))
  (bind _asbp_player_controller (Utilities|Casting|CastToBP_PlayerController (Components|GetOwner (Variables|/Script/Engine.Pawn|GetPlayerState _asbp_character))))
  (Variables|Default|SetAs%20BP%20Player%20Controller _asbp_player_controller)
  (CallFunction|PushExampleWidgettoStackLayer))

(event OnComponentEndOverlap(Box)
  (params (OverlappedComponent :type Primitive%20Component%20Object%20Reference) (OtherActor :type Actor%20Object%20Reference) (OtherComp :type Primitive%20Component%20Object%20Reference) (OtherBodyIndex :type Integer))
  (bind _w_example (Variables|Default|GetW_Example))
  ;[1 1 1] It is not used, just for example
  (Utilities|Casting|CastToBP_Character OtherActor)
  (Widget|Panel|ClearChildren (Variables|/Game/UI/Widgets/W_Example.W_Example_C|GetHorizontalBox_Dummies _w_example))
  (Default|RemoveWIdgetfromStackLayer (Variables|/Game/Core/BP_PlayerController.BP_PlayerController_C|GetW_MainLayers (Variables|Default|GetAs%20BP%20Player%20Controller)) "(TagName=\"UI.Layer.Game\")" _w_example))

(event Custom|Push%20Example%20Widget%20To%20Stack%20Layer
  (bind _as_bp_player_controller (Variables|Default|GetAs%20BP%20Player%20Controller))
  (bind _w_mainlayers (Variables|/Game/Core/BP_PlayerController.BP_PlayerController_C|GetW_MainLayers _as_bp_player_controller))
  (Default|PushWidgettoStackLayer _w_mainlayers "(TagName=\"UI.Layer.Game\")" "/Game/UI/Widgets/W_Example.W_Example_C")
  (bind _asw_example (Utilities|Casting|CastToW_Example (Class|CommonActivatableWidgetContainerBase|GetActiveWidget (Variables|/Game/UI/Widgets/W_MainLayers.W_MainLayers_C|GetStack_GameLayer _w_mainlayers))))
  (bind _output_get (Variables|Default|SetW_Example _asw_example))
  (Variables|/Game/UI/Widgets/W_Example.W_Example_C|SetWidgetCount _output_get (Variables|Default|GetWidgetCount))
  (CallFunction|AddDummyWidgets))

(event Custom|Add%20Dummy%20Widgets
  (for _index (range 0 (Variables|Default|GetWIdgetCount))
    (bind _returnvalue (UserInterface|CreateWidget "/Game/UI/Widgets/W_Dummy.W_Dummy_C" (Variables|Default|GetAs%20BP%20Player%20Controller)))
    (Class|HorizontalBox|AddChildtoHorizontalBox (Variables|/Game/UI/Widgets/W_Example.W_Example_C|GetHorizontalBox_Dummies (Variables|Default|GetW_Example)) _returnvalue))
  (CallFunction|UpdateDummyWidgetsVM))

(event Custom|Update%20Dummy%20Widgets%20VM
  ;[1 1 1] Update Dummy Numbers and get ViewModel using "Create Instance" creation type
  (for (_array_element _array_index) (Class|PanelWidget|GetAllChildren (Variables|/Game/UI/Widgets/W_Example.W_Example_C|GetHorizontalBox_Dummies (Variables|Default|GetW_Example)))
    (bind _asw_dummy (Utilities|Casting|CastToW_Dummy _array_element))
    (Variables|/Game/UI/Data/ViewModels/VM_Dummy.VM_Dummy_C|SetDummyNum (Variables|/Game/UI/Widgets/W_Dummy.W_Dummy_C|GetVM_Dummy _asw_dummy) _array_index)))

(event EventBeginPlay)

(fn ConstructionScript)