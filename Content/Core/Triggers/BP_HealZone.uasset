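; Trigger volume that gradually heals a BP_Character standing inside its box.
; Overlap begin stores the character and starts a looping one-second timer, which adds a small random amount of health while it is below max, without clamping the result.
; Overlap end by any BP_Character clears the timer; only the last character to enter is tracked.
; Start and stop print debug messages.
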(event OnComponentBeginOverlap(Box)
  (params (OverlappedComponent :type Primitive%20Component%20Object%20Reference) (OtherActor :type Actor%20Object%20Reference) (OtherComp :type Primitive%20Component%20Object%20Reference) (OtherBodyIndex :type Integer) (bFromSweep :type Boolean) (SweepResult :type Hit%20Result%20Structure%20%28by%20ref%29))
  (bind _asbp_character (Utilities|Casting|CastToBP_Character OtherActor))
  (Variables|Default|SetAs%20BP%20Character _asbp_character)
  (CallFunction|StartHeal))

(event OnComponentEndOverlap(Box)
  (params (OverlappedComponent :type Primitive%20Component%20Object%20Reference) (OtherActor :type Actor%20Object%20Reference) (OtherComp :type Primitive%20Component%20Object%20Reference) (OtherBodyIndex :type Integer))
  (Utilities|Casting|CastToBP_Character OtherActor)
  (CallFunction|StopHeal))

(event Custom|Start%20Heal
  (bind _returnvalue (Utilities|Time|SetTimerbyEvent (EventDispatchers|CreateEvent :!event Custom|Heal) 1.0 true))
  (Variables|Default|SetHeal%20Timer%20Handle _returnvalue)
  (Development|PrintString "Start Heal" true true "(R=0.023636,G=0.875000,B=0.000000,A=1.000000)" 5.0))

(event Custom|Heal
  (bind _as_bp_character (Variables|Default|GetAs%20BP%20Character))
  (if (< (Variables|/Game/Core/BP_Character.BP_Character_C|GetCurrent%20Health _as_bp_character) (Variables|/Game/Core/BP_Character.BP_Character_C|GetMax%20Health _as_bp_character))
    (Default|SetCurrentHealth _as_bp_character (+ (Variables|/Game/Core/BP_Character.BP_Character_C|GetCurrent%20Health _as_bp_character) (Math|Random|RandomIntegerinRange 1 15)))))

(event Custom|Stop%20Heal
  (Utilities|Time|ClearandInvalidateTimerbyHandle (Variables|Default|GetHeal%20Timer%20Handle))
  (Development|PrintString "Heal Stop" true true "(R=1.000000,G=0.521062,B=0.000000,A=1.000000)" 5.0))

(event EventBeginPlay)

(fn ConstructionScript)